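; BP_Alpinist is an actor with a skeletal alpinist that travels along the points of a referenced path spline.
; BeginPlay teleports the capsule to the current spline point.
; Each Tick advances the point index within 30 units, then moves the capsule toward that point without sweep.
; The world-space direction is applied as a local offset and normalized after delta-time scaling, so each step is one unit per frame.
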(event `self.ReceiveBeginPlay`
  (`SceneComponent.K2_SetWorldLocation` (`self.Capsule`) (`SplineComponent.GetLocationAtSplinePoint` (`/Game/BP_Path.Spline` (`self.path`)) (`self.currentControlPoint`) "World") false true))

(event `self.ReceiveTick`
  (params (DeltaSeconds :type "Float (single-precision)"))
  (bind _returnvalue (- (`SplineComponent.GetLocationAtSplinePoint` (`/Game/BP_Path.Spline` (`self.path`)) (`self.currentControlPoint`) "World") (`SceneComponent.K2_GetComponentLocation` (`self.SK_Alpinist_01`))))
  (if (not (> (`KismetMathLibrary.VSize` _returnvalue) 30.0))
    (bind _result (`/Engine/EditorBlueprintResources/StandardMacros.IncrementInt` (`self.currentControlPoint`))
      (:`  `
        (set `self.currentControlPoint` _result))))
  (`SceneComponent.K2_AddLocalOffset` (`self.Capsule`) (`KismetMathLibrary.Normal` (* _returnvalue DeltaSeconds)) false false))

(fn `UserConstructionScript`)