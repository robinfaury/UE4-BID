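; BP_Spawn_Alpinist is a spawner that continuously creates BP_Alpinist actors at the start of a referenced spline.
; On Tick, it compares game time with the last spawn time and spawns a new alpinist whenever more than a second has passed.
; Each alpinist receives the spline as its path, plus hard-coded climb trigger and hold spacing distances.
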(event `self.ReceiveTick`
  (params (DeltaSeconds :type "Float (single-precision)"))
  (bind _returnvalue (`KismetSystemLibrary.GetGameTimeInSeconds`))
  (if (> (- _returnvalue (`self.lastSpawn`)) 1.0)
    (set `self.lastSpawn` _returnvalue)
    (bind _returnvalue_2 (`|SpawnActorFromClass` "/Game/BP_Alpinist.BP_Alpinist_C" (`SplineComponent.GetTransformAtSplinePoint` (`/Game/BP_Path.Spline` (`self.Spline`)) 0 "World" false) "Undefined" "OverrideRootScale"))
    (set `/Game/BP_Alpinist.path` (`self.Spline`) _returnvalue_2)
    (set `/Game/BP_Alpinist.distTriggerClimb` 70.0 _returnvalue_2)
    (set `/Game/BP_Alpinist.distBetweenPrise` 20.0 _returnvalue_2)))

(fn `UserConstructionScript`)